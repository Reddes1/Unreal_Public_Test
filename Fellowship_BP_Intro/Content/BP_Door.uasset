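; Interactive door actor that the player swings open and closed with E while inside its trigger box.
; Box overlap enables and disables input on the actor for player controller 0, without checking what overlapped.
; When not locked, a FlipFlop plays or reverses a timeline that lerps the door mesh's relative rotation, with debug prints.
; The construction script tints the point light red or green from IsLocked, which nothing here changes.
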(event OnComponentBeginOverlap(Box)
  (params (OverlappedComponent :type Primitive%20Component%20Object%20Reference) (OtherActor :type Actor%20Object%20Reference) (OtherComp :type Primitive%20Component%20Object%20Reference) (OtherBodyIndex :type Integer) (bFromSweep :type Boolean) (SweepResult :type Hit%20Result%20Structure%20%28by%20ref%29))
  (Input|EnableInput (Game|GetPlayerController 0)))

(event OnComponentEndOverlap(Box)
  (params (OverlappedComponent :type Primitive%20Component%20Object%20Reference) (OtherActor :type Actor%20Object%20Reference) (OtherComp :type Primitive%20Component%20Object%20Reference) (OtherBodyIndex :type Integer))
  (Input|DisableInput (Game|GetPlayerController 0)))

(event Custom|ChangeLightColour
  (Rendering|Components|Light|SetLightColor (Variables|Default|GetPointLight) (Math|Color|SelectColor "(R=1.000000,G=0.071750,B=0.051854,A=1.000000)" "(R=0.292038,G=1.000000,B=0.197105,A=1.000000)" (Variables|Default|GetIsLocked)) true))

(event Input|KeyboardEvents|E
  (params (Key :type Key%20Structure :default "None"))
  (:Pressed
    (Development|PrintString "E Pressed")
    (if (not (Variables|Default|GetIsLocked))
      (Utilities|FlowControl|FlipFlop
        (:A
          (bind _door_rotation_alpha (Timeline|Open/Close%20Door Play)
            (:Update
              (Development|PrintString (Utilities|String|ToString(Float) _door_rotation_alpha))
              (Transformation|SetRelativeRotation (Variables|Default|GetSM_Door) (Math|Rotator|Lerp(Rotator) "0, 0, 0" "0.000000,100.000000,0.000000" _door_rotation_alpha) false false))))
        (:B
          (Timeline|Open/Close%20Door Reverse))))))

(fn ConstructionScript
  (CallFunction|ChangeLightColour))